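; Game mode Blueprint for ToonTanks that handles the UI response to game start and game over.
; StartGame shows the mouse cursor, and GameOver shows it again, then branches on WonGame to add the Won widget or, on a loss, a widget with no class set.
; Start screen, life bar and end-game text widget logic remains in the graph but is disconnected and never runs.
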(event `self.StartGame`
  (set `PlayerController.bShowMouseCursor` true (`GameplayStatics.GetPlayerController` 0)))

(event `self.GameOver`
  (params (bWonGame :type Boolean))
  (set `PlayerController.bShowMouseCursor` true (`GameplayStatics.GetPlayerController` 0))
  (if bWonGame
    (bind _returnvalue (`|CreateWidget` "/Game/Blueprints/Widgets/Won.Won_C"))
    (`UserWidget.AddToViewport` _returnvalue 0)
    (else
      (bind _returnvalue_2 (`|CreateWidget` "/Game/Blueprints/Widgets/Retry.Retry_C"))
      (`UserWidget.AddToViewport` _returnvalue_2 0))))

(fn `UserConstructionScript`)